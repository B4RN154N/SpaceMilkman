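; EndPoint is the level goal actor that sends the game to the WinState level once no Milk actors remain.
; On any overlap it counts Milk actors; if some are left, it unhides actors tagged MissingMilk, then hides them again when the overlap ends.
; The construction script snaps the actor to Y = 0, keeping its X and Z, which locks it to a single plane.
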(event `self.ReceiveActorBeginOverlap`
  (params (OtherActor :type "Actor Object Reference"))
  (if true
    (bind _outactors (`GameplayStatics.GetAllActorsOfClass` "/Game/Blueprints/Milk.Milk_C"))
    (if (== (`KismetArrayLibrary.Array_LastIndex` _outactors) -1)
      (`GameplayStatics.OpenLevel` "WinState")
      (else
        (bind _outactors_2 (`GameplayStatics.GetAllActorsWithTag` "MissingMilk"))
        (`self.SetActorHiddenInGame` _outactors_2 false)))))

(event `self.ReceiveActorEndOverlap`
  (params (OtherActor :type "Actor Object Reference"))
  (bind _outactors (`GameplayStatics.GetAllActorsWithTag` "MissingMilk"))
  (`self.SetActorHiddenInGame` _outactors true))

(fn `UserConstructionScript`
  (`self.K2_SetActorLocation` (`KismetMathLibrary.MakeVector` (.x (`self.K2_GetActorLocation`)) 0.0 (.z (`self.K2_GetActorLocation`)))))