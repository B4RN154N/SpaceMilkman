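; IceFloor is a floor actor that makes the player character slide like on ice while standing in it.
; When a MyCharacter2 overlaps SafetyCollider, it plays the PossessPlayer sound and zeroes the character movement's ground friction, braking friction factor and walking braking deceleration.
; The actor's end-overlap event sets those values back to hard-coded defaults instead of the character's previous settings.
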(event `self.SafetyCollider.OnComponentBeginOverlap`
  (params (OverlappedComponent :type "PrimitiveComponent Object Reference") (OtherActor :type "Actor Object Reference") (OtherComp :type "PrimitiveComponent Object Reference") (OtherBodyIndex :type Integer) (bFromSweep :type Boolean) (SweepResult :type "HitResult Structure (by ref)"))
  (bind _asmy_character_2 (cast `/Game/Blueprints/MyCharacter2` OtherActor))
  (`GameplayStatics.PlaySoundAtLocation` "/Engine/EditorSounds/GamePreview/PossessPlayer.PossessPlayer" (`self.K2_GetActorLocation`))
  (bind _charactermovement (`Character.CharacterMovement` _asmy_character_2))
  (set `CharacterMovementComponent.GroundFriction` 0.0 _charactermovement)
  (set `CharacterMovementComponent.BrakingFrictionFactor` 0.0 _charactermovement)
  (set `CharacterMovementComponent.BrakingDecelerationWalking` 0.0 _charactermovement))

(event `self.ReceiveActorEndOverlap`
  (params (OtherActor :type "Actor Object Reference"))
  (bind _asmy_character_2 (cast `/Game/Blueprints/MyCharacter2` OtherActor))
  (bind _charactermovement (`Character.CharacterMovement` _asmy_character_2))
  (set `CharacterMovementComponent.GroundFriction` 8.0 _charactermovement)
  (set `CharacterMovementComponent.BrakingFrictionFactor` 2.0 _charactermovement)
  (set `CharacterMovementComponent.BrakingDecelerationWalking` 2048.0 _charactermovement))

(fn `UserConstructionScript`)