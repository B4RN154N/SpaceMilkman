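; Jetpack pickup Blueprint that grants the player a jetpack-like boost when touched.
; Overlap of its JetPackSprite component by MyCharacter plays a powerup sound, destroys the sprite component and prints an activation message.
; It then raises the player character's jump hold time and air control and sets CollectedJetpack on the overlapping character.
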(event `self.JetPackSprite.OnComponentBeginOverlap`
  (params (OverlappedComponent :type "PrimitiveComponent Object Reference") (OtherActor :type "Actor Object Reference") (OtherComp :type "PrimitiveComponent Object Reference") (OtherBodyIndex :type Integer) (bFromSweep :type Boolean) (SweepResult :type "HitResult Structure (by ref)"))
  (bind _returnvalue (`GameplayStatics.GetPlayerCharacter` 0))
  (bind _asmy_character (cast `/Game/Blueprints/MyCharacter` OtherActor))
  (`GameplayStatics.PlaySoundAtLocation` "/Game/Audio/Powerup.Powerup" (`self.K2_GetActorLocation`))
  (`ActorComponent.K2_DestroyComponent` (`self.JetPackSprite`))
  (`KismetSystemLibrary.PrintString` "Jetpack Activated")
  (set `Character.JumpMaxHoldTime` 1.0 _returnvalue)
  (set `CharacterMovementComponent.AirControl` 0.8 (`Character.CharacterMovement` _returnvalue))
  (set `/Game/Blueprints/MyCharacter.collectedJetpack` true _asmy_character))

(fn `UserConstructionScript`)