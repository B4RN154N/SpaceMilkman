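; A 2D lift that moves its sprite between its origin and an editable end location on a timeline, with play rate derived from travel time.
; Each finished run waits a stop delay, then restarts in the opposite direction.
; A safety collider overlapped by the player character plays or reverses an active timeline, depending on whether it is playing.
; The construction script applies the tint and can preview the end position.
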(event `self.ReceiveBeginPlay`
  (`TimelineComponent.SetPlayRate` (`self.LiftTimeline`) (/ 1.0 (`self.TravelTimeInSeconds`)))
  (set `self.TestEndLocation` true))

(event `self.SafetyCollider.OnComponentBeginOverlap`
  (params (OverlappedComponent :type "PrimitiveComponent Object Reference") (OtherActor :type "Actor Object Reference") (OtherComp :type "PrimitiveComponent Object Reference") (OtherBodyIndex :type Integer) (bFromSweep :type Boolean) (SweepResult :type "HitResult Structure (by ref)"))
  (bind _lifttimeline (`self.LiftTimeline`))
  (cast `/Game/Blueprints/MyCharacter` OtherActor)
  (if (`ActorComponent.IsActive` _lifttimeline)
    (if (`TimelineComponent.IsPlaying` _lifttimeline)
      (bind (_direction _lerpalpha) (`Timeline|LiftTimeline` :!label _label)
        (:`Update`
          (`SceneComponent.K2_SetRelativeLocation` (`self.LiftSprite`) (`KismetMathLibrary.VLerp` (0.0 0.0 0.0) (`self.EndLocation`) _lerpalpha) false false))
        (:`Finished`
          (`KismetSystemLibrary.Delay` (`self.StopDelay`))
          (switch `ETimelineDirection` _direction
            (:`Forward`
              (`self.LiftBackward`))
            (:`Backward`
              (`self.LiftForward`)))))
      (else
        (goto _label :!via `Reverse`)))))

(event `LiftForward`
  (goto _label :!via `PlayFromStart`))

(event `LiftBackward`
  (goto _label :!via `ReverseFromEnd`))

(fn `UserConstructionScript`
  (bind _liftsprite (`self.LiftSprite`))
  (`SceneComponent.K2_SetRelativeLocation` _liftsprite (`KismetMathLibrary.SelectVector` (`self.EndLocation`) (0.0 0.0 0.0) (`self.TestEndLocation`)) false false)
  (`PaperSpriteComponent.SetSpriteColor` _liftsprite (`self.LiftColor`)))